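; Race tracker for the car racing game that runs the checkpoint sequence and lap logic for a track.
; On BeginPlay it passes lap count, save slot, map name and medal and best times to the custom player controller, then numbers and binds its checkpoints.
; Each cleared checkpoint plays a sound, activates the next and sets the respawn transform.
; The last one updates the lap or flags race completion, which triggers a controller restart.
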(event `self.ReceiveBeginPlay`
  ;[1 1 1] Event Begin Play, Get Controller Refrence & Pass values From Tracker To Controller and Sart The Checkpoint Sequence
  (bind _ascustom_player_controller (cast `/Game/BP_CarRacing/Custom_PlayerController` (`GameplayStatics.GetPlayerController` 0)))
  (set `self.RefOfCustomPlayerController` _ascustom_player_controller)
  (`self.ApplySettings`)
  (`self.StartSequence`))

(event `ApplySettings`
  (bind _refofcustomplayercontroller (`self.RefOfCustomPlayerController`))
  ;[1 1 1] Applying User Setttings When Starting Game. (Passing Custom Setting Values to The Controller e.g. MaxLap/Times Value etc.)
  (set `/Game/BP_CarRacing/Custom_PlayerController.MaxLaps` (`self.MaxLaps`) _refofcustomplayercontroller)
  (set `/Game/BP_CarRacing/Custom_PlayerController.SaveSlot` (`self.SaveGameName`) _refofcustomplayercontroller)
  (set `/Game/BP_CarRacing/Custom_PlayerController.NameOfMap` (`self.NameOfMap`) _refofcustomplayercontroller)
  (`self.UpdateTimes`)
  (`/Game/BP_CarRacing/Custom_PlayerController.StartGameSetup` _refofcustomplayercontroller))

(event `StartSequence`
  (bind _checkpoints (`self.Checkpoints`))
  ;[1 1 1] Start Sequence / Get All Checkpoint & Activate the First &Bind Event To Checkpoint Cleared
  (for (_array_element _array_index) (`self.Checkpoints`)
    (set `/Game/BP_CarRacing/BP_CheckPoint.CheckpointNumber` (+ _array_index 1) _array_element)
    (set `self.TotalCheckPoints` (`KismetArrayLibrary.Array_Length` _checkpoints))
    (`self.ActivateCheckpoint` (`|GetArrayItem` _checkpoints))
    (for _array_element_2 (`self.Checkpoints`)
      (add `/Game/BP_CarRacing/BP_CheckPoint.CheckpointCleared` _array_element_2 (delegate `CheckCheckpointCleared`)))))

(event `CheckCheckpointCleared`
  (params (NextCheckpoint :type Integer))
  (bind _refofcustomplayercontroller (`self.RefOfCustomPlayerController`))
  ;[1 1 1] Checkpoint Cleared - Check and See if Race is Over, If so. Restart the Race.
  (`self.LapCheck` NextCheckpoint)
  (`AudioComponent.Play` (`AmbientSound.AudioComponent` (`self.CheckpointSoundFX`)) 0.0)
  (if (`/Game/BP_CarRacing/Custom_PlayerController.RaceComplete` _refofcustomplayercontroller)
    (`/Game/BP_CarRacing/Custom_PlayerController.Restart` _refofcustomplayercontroller)))

(fn `ActivateCheckpoint`
  (params (NextCheckpoint :type "/Game/BP_CarRacing/BP_CheckPoint Object Reference"))
  (bind _trigger (`/Game/BP_CarRacing/BP_CheckPoint.Trigger` NextCheckpoint))
  ;[1 1 1] Activating The Next Checkpoint & Setting Overlap To True For Events
  (`SceneComponent.SetHiddenInGame` _trigger false false)
  (`SceneComponent.SetHiddenInGame` (`/Game/BP_CarRacing/BP_CheckPoint.ParticleSystem` NextCheckpoint) false false)
  (set `PrimitiveComponent.bGenerateOverlapEvents` true _trigger))

(fn `LapCheck`
  (params (Checkpoint :type Integer))
  (locals (LocalCheckpoint :type Integer))
  ;[1 1 1] Lap Check Script, Check If we Completed a Race / Lap Or Set Up a Next Checkpoint. Get Previous Checkpoint Location To respawn the Vechicle If Player Flip it
  (bind _output_get (set `local.LocalCheckpoint` Checkpoint))
  (if (== _output_get (`self.TotalCheckPoints`))
    (bind _isracecomplete_ (`self.RaceComplete`))
    (if (not _isracecomplete_)
      (`self.ActivateCheckpoint` (`|GetArrayItem` (`self.Checkpoints`))) ; Activating the First Checkpoint If Race isn't get Completed yet and Update the count of Lap
    )
    (`/Game/BP_CarRacing/Custom_PlayerController.UpdateLap` (`self.RefOfCustomPlayerController`))
    (else
      (`self.ActivateCheckpoint` (`|GetArrayItem` (`self.Checkpoints`) (`local.LocalCheckpoint`)))))
  (set `/Game/BP_CarRacing/Custom_PlayerController.RespawnLocation` (`self.GetTransform` (`|GetArrayItem` (`self.Checkpoints`) (- (`local.LocalCheckpoint`) 1))) (`self.RefOfCustomPlayerController`)) ; Executing It Still after "update lap" Because maybe player flip the car as it cross the last checkpoint
)

(fn `RaceComplete`
  (returns (`IsRaceComplete?` :type Boolean))
  (locals (LocalRaceComplete :type Boolean))
  (bind _refofcustomplayercontroller (`self.RefOfCustomPlayerController`))
  (bind _refofcustomplayercontroller_2 (`self.RefOfCustomPlayerController`))
  ;[1 1 1] Check if Race is Complete & Setting the Controller Varibale "Race Complete"
  (if (>= (`/Game/BP_CarRacing/Custom_PlayerController.ActualLap` _refofcustomplayercontroller_2) (`/Game/BP_CarRacing/Custom_PlayerController.MaxLaps` _refofcustomplayercontroller_2))
    (bind _output_get (set `/Game/BP_CarRacing/Custom_PlayerController.RaceComplete` true _refofcustomplayercontroller))
    (set `local.LocalRaceComplete` _output_get)
    (else
      (bind _output_get_2 (set `/Game/BP_CarRacing/Custom_PlayerController.RaceComplete` false _refofcustomplayercontroller))
      (set `local.LocalRaceComplete` _output_get_2)))
  (return (`local.LocalRaceComplete`)))

(fn `UpdateTimes`
  (bind _refofcustomplayercontroller (`self.RefOfCustomPlayerController`))
  ;[1 1 1] Passing Time Values From Tracker to Custom Player Controller For Processing
  (set `/Game/BP_CarRacing/Custom_PlayerController.GoldTime` (`self.GoldTime`) _refofcustomplayercontroller)
  (set `/Game/BP_CarRacing/Custom_PlayerController.SilverTime` (`self.SilverTime`) _refofcustomplayercontroller)
  (set `/Game/BP_CarRacing/Custom_PlayerController.BronzeTime` (`self.BronzeTime`) _refofcustomplayercontroller)
  (set `/Game/BP_CarRacing/Custom_PlayerController.BestLapTime` (`self.DefaultBestLap`) _refofcustomplayercontroller)
  (set `/Game/BP_CarRacing/Custom_PlayerController.BestRaceTime` (`self.DefaultBestTime`) _refofcustomplayercontroller))

(fn `UserConstructionScript`)