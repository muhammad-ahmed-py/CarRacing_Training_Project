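; BP_CheckPoint is a numbered race checkpoint that a car clears by driving through it in the intended direction.
; When a VehicleBlueprint stops overlapping the Trigger, a dot product of its velocity with the Arrow's forward vector confirms the direction.
; A valid pass fires the CheckpointCleared dispatcher with CheckpointNumber, hides the trigger and particle effect, and disables overlap events so it cannot clear again.
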(event `self.Trigger.OnComponentEndOverlap`
  (params (OverlappedComponent :type "PrimitiveComponent Object Reference") (OtherActor :type "Actor Object Reference") (OtherComp :type "PrimitiveComponent Object Reference") (OtherBodyIndex :type Integer))
  (bind _trigger (`self.Trigger`))
  ;[1 1 1] Checkpoint System Cleared, When Overlaping End
  (bind _asvehicle_blueprint (cast `/Game/VehicleAdvBP/Blueprints/VehicleBlueprint` OtherActor))
  (if (> (`KismetMathLibrary.Dot_VectorVector` (`self.GetVelocity` _asvehicle_blueprint) (`KismetMathLibrary.Conv_RotatorToVector` (`SceneComponent.K2_GetComponentRotation` (`self.Arrow`)))) 0.0)
    (`self.CheckpointCleared` (`self.CheckpointNumber`))
    (`SceneComponent.SetHiddenInGame` _trigger true false)
    (`SceneComponent.SetHiddenInGame` (`self.ParticleSystem`) true false)
    (set `PrimitiveComponent.bGenerateOverlapEvents` false _trigger)))

(fn `UserConstructionScript`)